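; AI spawner actor that populates the level with random pawns from BPAI, running behavior tree BT_A, up to the game mode's AI limit.
; On authority, BeginPlay starts a looping NoticeToGM timer only if DT_AI lacks an "AI" row.
; Each successful check spawns at a nearby random navigable point at the spawner's height, increments the game mode's count and resets the timer as one-shot, so the chain ends at the cap.
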(event EventBeginPlay
  (CallFunction|Initialize)
  (Networking|SwitchHasAuthority
    (:Authority
      (bind _returnvalue (Class|DataTableFunctionLibrary|DoesDataTableRowExist "/Game/ShootingGame/AI/AI_Data/DT_AI.DT_AI" (Variables|Default|GetAI)))
      (if (not _returnvalue)
        (Utilities|Time|SetTimerbyFunctionName 0 "NoticeToGM" 2.0 true)))))

(fn ConstructionScript)

(fn SpawnAI
  (bind _randomlocation (Class|NavigationSystemV1|GetRandomLocationinNavigableRadius (Transformation|GetActorLocation) 5e+02 0 0))
  (AI|SpawnAIFromClass (.OutItem (Utilities|Array|Random (Variables|Default|GetBP_AI))) "/Game/ShootingGame/AI/AI_BT/BT_A.BT_A" (Math|Vector|MakeVector (.x _randomlocation) (.y _randomlocation) (.z (Transformation|GetActorLocation))) "0, 0, 0" false 0))

(fn NoticetoGM
  (bind _shootinggm_ref (Variables|Default|GetShootingGM_REF))
  (if (< (Variables|/Game/ShootingGame/GameMode/BP_ShootingGameMode.BP_ShootingGameMode_C|GetAI_Alive _shootinggm_ref) (Variables|/Game/ShootingGame/GameMode/BP_ShootingGameMode.BP_ShootingGameMode_C|GetAI_Max _shootinggm_ref))
    (CallFunction|SpawnAI)
    (Default|IncreaseAI _shootinggm_ref)
    (Utilities|Time|SetTimerbyFunctionName 0 "NoticeToGM" 2.0)))

(fn Initialize
  (bind _asbp_shooting_game_mode (Utilities|Casting|CastToBP_ShootingGameMode (Game|GetGameMode)))
  (Variables|Default|SetShootingGM_REF _asbp_shooting_game_mode))