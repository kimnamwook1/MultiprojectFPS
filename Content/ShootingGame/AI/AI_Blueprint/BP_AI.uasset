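; BP_AI is a damageable AI actor in the shooting game, with clamped HP and an item drop routine.
; Its health widget is bound to the AI, shows while the player character overlaps its sphere, and yaws toward the player every tick.
; SpawnItem, not called within this file, spawns a weapon spawner and random pickups nearby, destroys the actor and decrements the game mode's AI count.
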(event OnComponentBeginOverlap(Sphere)
  (params (OverlappedComponent :type Primitive%20Component%20Object%20Reference) (OtherActor :type Actor%20Object%20Reference) (OtherComp :type Primitive%20Component%20Object%20Reference) (OtherBodyIndex :type Integer) (bFromSweep :type Boolean) (SweepResult :type Hit%20Result%20Structure%20%28by%20ref%29))
  (Utilities|Casting|CastToBP_ShootingCharacter OtherActor)
  (Rendering|SetVisibility (Variables|Default|GetAIHealthWidget) true false))

(event OnComponentEndOverlap(Sphere)
  (params (OverlappedComponent :type Primitive%20Component%20Object%20Reference) (OtherActor :type Actor%20Object%20Reference) (OtherComp :type Primitive%20Component%20Object%20Reference) (OtherBodyIndex :type Integer))
  (Utilities|Casting|CastToBP_ShootingCharacter OtherActor)
  (Rendering|SetVisibility (Variables|Default|GetAIHealthWidget) false false))

(event EventBeginPlay
  (bind _asbp_shooting_game_mode (Utilities|Casting|CastToBP_ShootingGameMode (Game|GetGameMode))
    (:then
      (Variables|Default|SetShootingGM_REF _asbp_shooting_game_mode)
      (CallFunction|WidgetInitialize))
    (:CastFailed
      (CallFunction|WidgetInitialize))))

(event EventTick
  (params (DeltaSeconds :type Float%20%28single-precision%29))
  (CallFunction|WidgetLookPlayer))

(fn ConstructionScript)

(fn AddDamage
  (params (Damage :type Float%20%28single-precision%29))
  (Variables|Default|SetHP (Math|Float|Clamp(Float) (- (Variables|Default|GetHP) Damage) 0.0 (Variables|Default|GetHP_Max))))

(fn SpawnItem
  (bind _returnvalue (Transformation|GetActorTransform))
  (Game|SpawnActorfromClass "/Game/ShootingGame/Blueprint/BP_WeaponSpawner.BP_WeaponSpawner_C" _returnvalue "AdjustIfPossibleButAlwaysSpawn" 0 0)
  (for _index (range 0 (Math|Random|RandomInteger 5))
    (bind _randomlocation (Class|NavigationSystemV1|GetRandomLocationinNavigableRadius (.Location (Math|Transform|BreakTransform _returnvalue)) 1e+02 0 0))
    (Game|SpawnActorfromClass "/Game/ShootingGame/Blueprint/BP_SpawnItem.BP_SpawnItem_C" (Math|Transform|MakeTransform _randomlocation "0, 0, 0" "1,1,1") "AlwaysSpawn" 0 0))
  (Actor|DestroyActor)
  (Default|DecreaseAI (Variables|Default|GetShootingGM_REF)))

(fn WidgetInitialize
  (bind _asaihealth_widget (Utilities|Casting|CastToAIHealthWidget (UserInterface|GetUserWidgetObject (Variables|Default|GetAIHealthWidget))))
  (bind _output_get (Variables|Default|SetAIHealth_Widget _asaihealth_widget))
  (Variables|/Game/ShootingGame/AI/AI_Widget/AIHealthWidget.AIHealthWidget_C|SetAI _output_get self))

(fn WidgetLookPlayer
  (Transformation|SetWorldRotation (Variables|Default|GetAIHealthWidget) (Math|Rotator|MakeRotator 0.0 0.0 (.yaw (Math|Rotator|FindLookatRotation (Transformation|GetWorldLocation (Variables|Default|GetAIHealthWidget)) (Transformation|GetActorLocation (Game|GetPlayerCharacter 0))))) false false))