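; Player state for a multiplayer shooting game, holding each player's HP, armor, name, kills and deaths.
; Damage drains armor first and spills into HP, while heal and armor functions clamp their values and a death check tests for zero HP.
; RepNotify functions relay changes through event dispatchers, and BeginPlay asks the first local controller's BP_ShootingHUD to bind to this state.
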(event EventBeginPlay
  (CallFunction|InitBind))

(fn ConstructionScript)

(fn AddDamage
  (params (Damage :type Float%20%28single-precision%29))
  (if (> (- (Variables|Default|GetArmor) Damage) 0.0)
    (Variables|Default|SetArmor (- (Variables|Default|GetArmor) Damage))
    (else
      (Variables|Default|SetHP (Math|Float|Clamp(Float) (+ (Variables|Default|GetHP) (- (Variables|Default|GetArmor) Damage)) 0.0 1e+02))
      (Variables|Default|SetArmor 0.0))))

(fn OnRepHP
  ;[1 1 1] Client(서버에서 순차적으로 보내는 것이 아니라 쌓이뒀다가 한번에 보낸다)
  (Development|PrintString (Utilities|String|Append "On Rep HP" (Utilities|String|ToString(Float) (Variables|Default|GetHP))) true true "(R=0.000000,G=0.660000,B=1.000000,A=1.000000)" 6e+01)
  (Default|CallEventDispatcherHP (Variables|Default|GetHP) 1e+02))

(fn AddHeal
  (params (Heal :type Float%20%28single-precision%29))
  (Variables|Default|SetHP (Math|Float|Clamp(Float) (+ Heal (Variables|Default|GetHP)) 0.0 1e+02)))

(fn OnRepArmor
  (Default|CallEventDispatcherArmor (Variables|Default|GetArmor) 1e+02))

(fn AddArmor
  (params (Armor :type Float%20%28single-precision%29))
  (Variables|Default|SetArmor (Math|Float|Clamp(Float) (+ (Variables|Default|GetArmor) Armor) 0.0 1e+02)))

(fn SetName
  (params (Name :type String))
  (bind _output_get (Variables|Default|SetName Name))
  (Development|PrintString _output_get))

(fn OnRepName
  (Default|CallEventDispatcherChangeName (Variables|Default|GetName)))

(fn InitBind
  (bind _asbp_shooting_hud (Utilities|Casting|CastToBP_ShootingHUD (HUD|GetHUD (Game|GetPlayerController 0)))
    (:then
      (Default|BindPlayerState _asbp_shooting_hud self))
    (:CastFailed
      (Development|PrintString "BP_Shooting HUD Test Fail" true true "(R=1.000000,G=0.027049,B=0.035007,A=1.000000)" 6e+01))))

(fn OnRepKill
  (Default|CallEventDispatcherKill (Variables|Default|GetKill)))

(fn OnRepDeath
  (Default|CallEventDispatcherDeath (Variables|Default|GetDeath)))

(fn AddKill
  (Variables|Default|SetKill (+ (Variables|Default|GetKill) 1)))

(fn AddDeath
  (Variables|Default|SetDeath (+ (Variables|Default|GetDeath) 1)))

(fn IsDeath
  (return (<= (Variables|Default|GetHP) 0.0)))