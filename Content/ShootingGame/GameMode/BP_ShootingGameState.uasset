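; Game state for the shooting game that spawns the magnetic field and decides each player's win or loss.
; On BeginPlay, the authority spawns BP_MagneticField at a random navigable point around a fixed origin and stores it.
; CurrentState's OnRep runs a winner check over PlayerArray.
; Through each player's controller, zero-HP players see Lose during Playing, and End Game shows everyone Win or Lose by HP.
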(event Custom|CheckWinner%28Server%29
  ;[1 0.2132 0.1913] CheckWinner
  (for _array_element (Variables|/Script/Engine.GameStateBase|GetPlayerArray (Game|GetGameState))
    (bind _asbp_shooting_player_state (Utilities|Casting|CastToBP_ShootingPlayerState _array_element))
    (switch Utilities|FlowControl|Switch|SwitchonEN-GameState (Variables|Default|GetCurrentState)
      (:NewEnumerator0
        (if (<= (Variables|/Game/ShootingGame/GameMode/BP_ShootingPlayerState.BP_ShootingPlayerState_C|GetHP _asbp_shooting_player_state) 0.0)
          (CallFunction|CheckWinner(Client) true _asbp_shooting_player_state)))
      (:NewEnumerator1
        (CallFunction|CheckWinner(Client) (<= (Variables|/Game/ShootingGame/GameMode/BP_ShootingPlayerState.BP_ShootingPlayerState_C|GetHP _asbp_shooting_player_state) 0.0) _asbp_shooting_player_state)))))

(event Custom|SpawnMF%28Server%29
  ;[9.495 1 1] Spawn MagneticField
  (CallFunction|SpawnMF))

(event Custom|CheckWinner%28Client%29
  (params (NewParam :type Boolean) (타깃 :type Actor%20Object%20Reference))
  (bind _returnvalue (Components|GetOwner 타깃))
  ;[1 0.2132 0.1913] CheckWinner
  (if NewParam
    (bind _asbp_shooting_player_controller (Utilities|Casting|CastToBP_ShootingPlayerController _returnvalue))
    (Default|ShowResultLose _asbp_shooting_player_controller)
    (else
      (bind _asbp_shooting_player_controller_2 (Utilities|Casting|CastToBP_ShootingPlayerController _returnvalue))
      (Default|ShowResultWin _asbp_shooting_player_controller_2))))

(event EventBeginPlay
  ;[9.495 1 1] Spawn MagneticField
  (Networking|SwitchHasAuthority
    (:Authority
      (CallFunction|SpawnMF(Server)))))

(fn ConstructionScript)

(fn OnRepCurrentState
  (CallFunction|CheckWinner(Server)))

(fn SpawnMF
  (bind _returnvalue (Math|Vector|MakeVector -6e+02 -4.4e+02 -4e+01))
  (bind _randomlocation (Class|NavigationSystemV1|GetRandomLocationinNavigableRadius (Math|Vector|MakeVector (.x _returnvalue) (.y _returnvalue) 0.0) 1e+04 0 0))
  (bind _returnvalue_2 (Game|SpawnActorfromClass "/Game/ShootingGame/BattleRoyaleCircle/BP_MagneticField.BP_MagneticField_C" (Math|Transform|MakeTransform (Math|Vector|MakeVector (.x _randomlocation) (.y _randomlocation) (.z _returnvalue)) "0, 0, 0" "1,1,1") "Undefined" 0 0))
  (Variables|Default|SetMField _returnvalue_2))