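; Player controller for the shooting game that handles player naming, character spawning and a text chat HUD.
; On possession it copies the GameInstance name to the PlayerState.
; Spawning passes the GameInstance's selected class to SpawnCharacterServer, which tags a PlayerStart "Found" but spawns and possesses at a random one.
; Chat messages fan out through the GameMode's ConnectPlayers list to each controller's ChatHUD, and Enter toggles chat input mode.
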(event Custom|SpawnCharacter
  (bind _asshooting_game_instance (Utilities|Casting|CastToShootingGameInstance (Game|GetGameInstance)))
  (CallFunction|SpawnCharacterServer (Variables|/Game/ShootingGame/GameMode/ShootingGameInstance.ShootingGameInstance_C|GetSelectedCharacter _asshooting_game_instance)))

(event Custom|SpawnCharacterServer
  (params (Class :type Character%20Class%20Reference))
  (bind _outactors (Actor|GetAllActorsOfClass "/Script/Engine.PlayerStart"))
  (bind _output_get (Variables|Default|SetPlayerStarts _outactors))
  (bind _array_element (Utilities|Array|ForEachLoopwithBreak _output_get :!label _label)
    (:LoopBody
      (if (Utilities|Name|NotEqual(Name) (Variables|/Script/Engine.PlayerStart|GetPlayerStartTag _array_element) "Found")
        (Variables|/Script/Engine.PlayerStart|SetPlayerStartTag _array_element "Found")
        (goto _label Break)))
    (:Completed
      (bind _returnvalue (Game|SpawnActorfromClass Class (Transformation|GetActorTransform (.OutItem (Utilities|Array|Random (Variables|Default|GetPlayerStarts)))) "AdjustIfPossibleButAlwaysSpawn" 0 0))
      (Pawn|Possess self _returnvalue))))

(event Custom|ResClientPossess
  (bind _asshooting_game_instance (Utilities|Casting|CastToShootingGameInstance (Game|GetGameInstance)))
  (CallFunction|ReqSetName (Variables|/Game/ShootingGame/GameMode/ShootingGameInstance.ShootingGameInstance_C|GetName _asshooting_game_instance)))

(event Custom|InitializeChatHUD
  ;[1 1 1] Setting ChatHUD
  (Development|PrintString "SettingHUD" false false)
  (bind _returnvalue (UserInterface|CreateWidget "/Game/ShootingGame/Widget/Chat/ChatHUDWidget.ChatHUDWidget_C" self))
  (bind _output_get (Variables|Default|SetChatHUDREF _returnvalue))
  (UserInterface|Viewport|AddtoViewport _output_get 0))

(event Custom|ReqSetName
  (params (NewName :type String))
  (bind _asbp_shooting_player_state (Utilities|Casting|CastToBP_ShootingPlayerState (Variables|GetPlayerState)))
  (Default|SetName _asbp_shooting_player_state NewName)
  ;[1 1 1] Setting ChatHUD
  (Variables|Default|SetPlayerName NewName))

(event Custom|UpdateChatLog
  (params (Sender :type String) (Message :type String))
  ;[1 1 1] ProcessChats
  (Default|UpdateChatLog (Variables|Default|GetChatHUDREF) (Utilities|Struct|MakeChatLogEntryStruct Sender Message)))

(event Custom|SendCheckMSG
  (params (Text :type String))
  ;[1 1 1] ProcessChats
  (bind _asbp_shooting_game_mode (Utilities|Casting|CastToBP_ShootingGameMode (Game|GetGameMode)))
  (for _array_element (Variables|/Game/ShootingGame/GameMode/BP_ShootingGameMode.BP_ShootingGameMode_C|GetConnectPlayers _asbp_shooting_game_mode)
    (CallFunction|UpdateChatLog _array_element (Variables|Default|GetPlayerName) Text)))

(event Custom|ToggleChat
  (params (MouseCursor :type Boolean))
  (if MouseCursor
    (Widget|SetVisibility (Variables|Default|GetChatHUDREF) "Visible")
    (Input|SetInputModeGameandUI self (Variables|/Game/ShootingGame/Widget/Chat/ChatHUDWidget.ChatHUDWidget_C|GetChatEntry (Variables|Default|GetChatHUDREF)) "DoNotLock" true)
    (Variables|Default|SetShowMouseCursor false)
    (else
      (Input|SetInputModeGameOnly self))))

(event EventBeginPlay
  (Input|SetInputModeGameOnly self)
  (CallFunction|InitializeChatHUD))

(event EventPossess
  (params (PossessedPawn :type Pawn%20Object%20Reference))
  (CallFunction|ResClientPossess))

(event Input|KeyboardEvents|Enter
  (params (Key :type Key%20Structure :default "None"))
  (:Pressed
    (Variables|/Game/ShootingGame/Widget/Chat/ChatHUDWidget.ChatHUDWidget_C|SetIsChatOn (Variables|Default|GetChatHUDREF) true)
    (bind _showcursor (CallFunction|ChatonOff))
    (Development|PrintString (Utilities|String|ToString(Boolean) _showcursor))
    (CallFunction|ToggleChat _showcursor)))

(fn ConstructionScript)

(fn ChatonOff
  (bind _output_get (Variables|Default|SetShowMouseCursor (not (Variables|Default|GetShowMouseCursor))))
  (if _output_get
    (bind _output_get_2 (Variables|Default|SetShowMouseCursor true))
    (return _output_get_2)
    (else
      (bind _output_get_3 (Variables|Default|SetShowMouseCursor false))
      (return _output_get_3))))