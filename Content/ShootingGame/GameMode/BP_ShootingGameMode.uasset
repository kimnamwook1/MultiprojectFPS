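; Game mode for a shooting game that handles player joins, AI population and match state.
; PostLogin registers each shooting controller, names it from a list, spawns its character and sets the survivor count from the player total.
; It tracks living AI and notifies BP_AISpawner when a decrease leaves the count below the maximum.
; BeginPlay, CountSurvivor and OnlyOneLeft each switch the GameState's state enum, starting from Ready.
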(event Custom|IncreaseAI
  ;[1 1 1] Control AINumvber
  (Variables|Default|SetAI_Alive (+ (Variables|Default|GetAI_Alive) 1)))

(event Custom|DecreaseAI
  ;[1 1 1] Control AINumvber
  (Variables|Default|SetAI_Alive (- (Variables|Default|GetAI_Alive) 1))
  (if (< (Variables|Default|GetAI_Alive) (Variables|Default|GetAI_Max))
    (bind _returnvalue (Actor|GetActorOfClass "/Game/ShootingGame/AI/AI_Blueprint/BP_AISpawner.BP_AISpawner_C"))
    (Default|NoticetoGM _returnvalue)))

(event Custom|CountSurvivor
  ;[1 1 1] 1명이라도 죽으면 CountSurvior을 호출하여 Enum Switch를 Playing으로 변경
  (Variables|/Game/ShootingGame/GameMode/BP_ShootingGameState.BP_ShootingGameState_C|SetCurrentState (Variables|Default|GetGS_Ref) "NewEnumerator0"))

(event Custom|OnlyOneLeft
  (Variables|/Game/ShootingGame/GameMode/BP_ShootingGameState.BP_ShootingGameState_C|SetCurrentState (Variables|Default|GetGS_Ref) "NewEnumerator1"))

(event EventPostLogin
  (params (NewPlayer :type Player%20Controller%20Object%20Reference))
  (bind _asbp_shooting_player_controller (Utilities|Casting|CastToBP_ShootingPlayerController NewPlayer))
  (bind _returnvalue (Utilities|Array|Add (Variables|Default|GetConnectPlayers) _asbp_shooting_player_controller))
  (Default|ReqSetName _asbp_shooting_player_controller (Utilities|Array|Get(acopy) (Variables|Default|GetplayerNames) _returnvalue))
  (Default|SpawnCharacter _asbp_shooting_player_controller)
  (bind _returnvalue_2 (Class|GameModeBase|GetNumPlayers))
  (Variables|Default|SetSurvivor _returnvalue_2))

(event EventBeginPlay
  ;[1 1 1 1 15] BeginPlay가 실행되면 GameState를 가져와서 변수로 만들고 GS의 Enum을 Switch를 Ready로 변경
  (bind _asbp_shooting_game_state (Utilities|Casting|CastToBP_ShootingGameState (Game|GetGameState)))
  (bind _output_get (Variables|Default|SetGS_Ref _asbp_shooting_game_state))
  (Variables|/Game/ShootingGame/GameMode/BP_ShootingGameState.BP_ShootingGameState_C|SetCurrentState _output_get "NewEnumerator2"))

(fn ConstructionScript)