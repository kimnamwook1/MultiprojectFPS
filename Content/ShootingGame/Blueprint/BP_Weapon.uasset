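; BP_Weapon is a networked, pick-up automatic hitscan rifle that reads mesh, damage and magazine size from WeaponRef.
; Pickup attaches it to the character's socket, dropping any held weapon and switching rotation mode.
; A looping timer replays fire montages; notify handlers play effects and have the owning player request a server line trace for damage.
; Ammo is predicted on clients, spent in the server hit check, refilled from character magazines, and shown on the HUD.
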(event Custom|ReqHitCheck
  (params (Location :type Vector :default "0.000000,0,0") (Forward :type Vector))
  ;[1 1 1] Server에서 HitCheck
  (Development|PrintString "ReqHitcheck" false false)
  (bind _hitlocation (CallFunction|ServerHitCheck Location Forward))
  (CallFunction|HitEffect _hitlocation))

(event Custom|ReqReload
  (CallFunction|ServerUseMag))

(event Custom|HitEffect
  (params (HitLocation :type Vector))
  (Effects|SpawnEmitteratLocation "/Game/MilitaryWeapDark/FX/P_RocketLauncher_Explosion_01.P_RocketLauncher_Explosion_01" HitLocation "0, 0, 0" "0.010000,0.010000,0.010000"))

(event EventBeginPlay
  (bind _weaponref (Variables|Default|GetWeaponRef))
  (Components|StaticMesh|SetStaticMesh (Variables|Default|GetStaticMesh) (.staticmesh _weaponref))
  (Variables|Default|SetAmmo (.maxammo _weaponref)))

(fn ConstructionScript)

(fn AttachtoCharacter
  (params (Character :type Character%20Object%20Reference))
  (bind _staticmesh (Variables|Default|GetStaticMesh))
  (Physics|SetSimulatePhysics _staticmesh false)
  (Collision|SetCollisionEnabled _staticmesh "QueryAndPhysics")
  (Transformation|AttachComponentToComponent (Variables|/Script/Engine.Character|GetMesh Character) "weapon" "SnapToTarget" "SnapToTarget" "KeepWorld" true)
  (bind _asbp_shooting_character (Utilities|Casting|CastToBP_ShootingCharacter Character))
  (bind _output_get (Variables|Default|SetOwnCharacter _asbp_shooting_character))
  (Variables|/Game/ShootingGame/GameMode/BP_ShootingCharacter.BP_ShootingCharacter_C|SetAttachedWeapon _output_get self)
  (Variables|/Script/Engine.Pawn|SetbUseControllerRotationYaw _asbp_shooting_character true)
  (Variables|/Script/Engine.CharacterMovementComponent|SetbOrientRotationToMovement (Variables|/Script/Engine.Character|GetCharacterMovement _asbp_shooting_character) false)
  (CallFunction|UpdateUIAmmo (Variables|Default|GetAmmo)))

(fn DetachfromCharacter
  (params (Character :type Character%20Object%20Reference))
  (Transformation|DetachFromActor "KeepWorld" "KeepWorld" "KeepWorld")
  (Collision|SetCollisionEnabled (Variables|Default|GetStaticMesh) "QueryAndPhysics")
  (Physics|SetSimulatePhysics (Variables|Default|GetStaticMesh) true)
  (CallFunction|UpdateUIAmmo)
  ;[1 1 1] Unequip상태로 정보 변경
  (bind _asbp_shooting_character (Utilities|Casting|CastToBP_ShootingCharacter Character))
  (Variables|/Game/ShootingGame/GameMode/BP_ShootingCharacter.BP_ShootingCharacter_C|SetAttachedWeapon _asbp_shooting_character 0)
  (Variables|Default|SetOwnCharacter 0)
  (Variables|/Script/Engine.Pawn|SetbUseControllerRotationYaw _asbp_shooting_character false)
  (Variables|/Script/Engine.CharacterMovementComponent|SetbOrientRotationToMovement (Variables|/Script/Engine.Character|GetCharacterMovement _asbp_shooting_character) true))

(fn PullTrigger
  (params (Character :type Character%20Object%20Reference))
  (Animation|PlayAnimMontage Character "/Game/anim/Fire_Rifle_Hip_Montage.Fire_Rifle_Hip_Montage" 1.0 "None")
  (Utilities|Time|SetTimerbyFunctionName 0 "AdditionalShot" 0.3 true))

(fn EventNotifyFire
  (bind _staticmesh (Variables|Default|GetStaticMesh))
  ;[1 1 1] Client
  (Networking|SwitchHasAuthority
    (:Authority
      (if (CallFunction|CanUseAmmo?)
        (Effects|SpawnEmitteratLocation "/Game/MilitaryWeapDark/FX/P_Pistol_MuzzleFlash_01.P_Pistol_MuzzleFlash_01" (Transformation|GetSocketLocation _staticmesh "Muzzle") (Transformation|GetSocketRotation _staticmesh "Muzzle") :!label _label)
        (Audio|Components|Audio|Play (Variables|Default|GetAudio) 0.0)
        (Utilities|CheckMyPlayer
          (:Ture
            (CallFunction|ReqHitCheck (Transformation|GetSocketLocation (Variables|Default|GetStaticMesh) "Muzzle") (Transformation|GetActorForwardVector (Game|GetPlayerCameraManager 0)))))))
    (:Remote
      (bind _isusedammo_ (CallFunction|UseAmmo))
      (if _isusedammo_
        (goto _label)))))

(fn AdditionalShot
  (bind _owncharacter (Variables|Default|GetOwnCharacter))
  (Utilities|IsValid _owncharacter
    (:Is%20Valid
      (Animation|PlayAnimMontage _owncharacter "/Game/anim/Fire_Rifle_Hip_Montage.Fire_Rifle_Hip_Montage" 1.0 "None"))
    (:Is%20Not%20Valid
      (Utilities|Time|ClearTimerbyFunctionName 0 "AdditionalShot"))))

(fn ReleaseTrigger
  (Utilities|Time|ClearTimerbyFunctionName 0 "AdditionalShot")
  (Utilities|Time|ClearTimerbyFunctionName 0 "PullTrigger"))

(fn UpdateUIAmmo
  (params (Ammo :type Integer))
  (Utilities|IsValid (Variables|Default|GetOwnCharacter)
    (:Is%20Valid
      (Utilities|CheckMyPlayer
        (:Ture
          (if true
            (bind _asbp_shooting_hud (Utilities|Casting|CastToBP_ShootingHUD (HUD|GetHUD (Game|GetPlayerController 0))))
            (Default|UpdateAmmo _asbp_shooting_hud Ammo)))))))

(fn UseAmmo
  (if (CallFunction|CanUseAmmo?)
    (bind _output_get (Variables|Default|SetAmmo (- (Variables|Default|GetAmmo) 1)))
    (CallFunction|UpdateUIAmmo _output_get)
    (return true)
    (else
      (return false))))

(fn SetAmmo
  (params (Ammo :type Integer))
  (bind _output_get (Variables|Default|SetAmmo Ammo))
  (CallFunction|UpdateUIAmmo _output_get))

(fn DoReload
  (bind _owncharacter (Variables|Default|GetOwnCharacter))
  (Utilities|IsValid _owncharacter
    (:Is%20Valid
      (if (Default|HasMag _owncharacter)
        (Animation|PlayAnimMontage _owncharacter "/Game/Rifle_Reload_2_Montage.Rifle_Reload_2_Montage" 1.0 "None")))))

(fn EventNotifyReload
  (Utilities|CheckMyPlayer
    (:Ture
      (CallFunction|ReqReload))))

(fn CanUseAmmo?
  ;[1 1 1] Ammo가 0보다 클때만 canuse true로 반환, 퓨어 켜줌
  (return (> (Variables|Default|GetAmmo) 0)))

(fn ServerHitCheck
  (params (Location :type Vector) (Forward :type Vector))
  (bind _isusedammo_ (CallFunction|UseAmmo))
  (if _isusedammo_
    (bind _outhit (Collision|LineTraceForObjects (+ Location (* Forward 0.0)) (+ Location (* Forward 3e+03)) (Utilities|Array|MakeArray "ObjectTypeQuery1" "ObjectTypeQuery2" "ObjectTypeQuery4" "ObjectTypeQuery5" "ObjectTypeQuery3" "ObjectTypeQuery6" "ObjectTypeQuery7") true (Utilities|Array|MakeArray (Variables|Default|GetOwnCharacter)) "Persistent"))
    (Utilities|FlowControl|Sequence
      (:then_0
        (bind _returnvalue (Game|Damage|ApplyDamage (.HitActor (Collision|BreakHitResult _outhit)) (.damage (Variables|Default|GetWeaponRef)) (Pawn|GetController (Variables|Default|GetOwnCharacter)) self))
        (bind _output_get (Variables|Default|SetWeaponDamage _returnvalue))
        (Development|PrintString (Utilities|String|Append "" "" "Damge : " (Utilities|String|ToString(Float) _output_get)))
        (return (.Location (Collision|BreakHitResult _outhit)))))))

(fn OnRepAmmo
  (CallFunction|UpdateUIAmmo (Variables|Default|GetAmmo)))

(fn ServerUseMag
  (bind _isusedmag (Default|UseMag (Variables|Default|GetOwnCharacter)))
  (if _isusedmag
    (CallFunction|SetAmmo (.maxammo (Variables|Default|GetWeaponRef)))))

(fn EventCanPickUp
  (return (not (Utilities|IsValid (Variables|Default|GetOwnCharacter)))))

(fn EventPress
  (params (Character :type Character%20Object%20Reference))
  (bind _asbp_shooting_character (Utilities|Casting|CastToBP_ShootingCharacter Character))
  (Utilities|IsValid (Variables|/Game/ShootingGame/GameMode/BP_ShootingCharacter.BP_ShootingCharacter_C|GetAttachedWeapon _asbp_shooting_character)
    (:Is%20Valid
      (CallFunction|DetachfromCharacter (Variables|/Game/ShootingGame/GameMode/BP_ShootingCharacter.BP_ShootingCharacter_C|GetAttachedWeapon _asbp_shooting_character) Character))
    (:Is%20Not%20Valid
      _))
  (CallFunction|AttachtoCharacter Character)
  (return true))

(fn EventRelease
  (params (Character :type Character%20Object%20Reference))
  (return true))