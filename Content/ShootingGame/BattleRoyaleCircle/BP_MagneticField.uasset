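; Battle royale magnetic field actor: a shrinking zone that tracks whether player 0 is inside it.
; On BeginPlay it calls the character's FuncDealMagneticField, enables mesh overlaps after a short delay, then runs a timeline shrinking X/Y at a fixed tall Z.
; Overlap begin and end set the character's IsInside flag.
; SetField and UpdateField provide randomly offset, lerped move-and-shrink steps, but are not called within this Blueprint.
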(event OnComponentBeginOverlap(StaticMesh)
  (params (OverlappedComponent :type Primitive%20Component%20Object%20Reference) (OtherActor :type Actor%20Object%20Reference) (OtherComp :type Primitive%20Component%20Object%20Reference) (OtherBodyIndex :type Integer) (bFromSweep :type Boolean) (SweepResult :type Hit%20Result%20Structure%20%28by%20ref%29))
  (if (== OtherActor (Game|GetPlayerCharacter 0))
    (bind _asbp_shooting_character (Utilities|Casting|CastToBP_ShootingCharacter (Game|GetPlayerCharacter 0)))
    (Variables|/Game/ShootingGame/GameMode/BP_ShootingCharacter.BP_ShootingCharacter_C|SetIsInside _asbp_shooting_character true)))

(event OnComponentEndOverlap(StaticMesh)
  (params (OverlappedComponent :type Primitive%20Component%20Object%20Reference) (OtherActor :type Actor%20Object%20Reference) (OtherComp :type Primitive%20Component%20Object%20Reference) (OtherBodyIndex :type Integer))
  (if (== OtherActor (Game|GetPlayerCharacter 0))
    (bind _asbp_shooting_character (Utilities|Casting|CastToBP_ShootingCharacter (Game|GetPlayerCharacter 0)))
    (Variables|/Game/ShootingGame/GameMode/BP_ShootingCharacter.BP_ShootingCharacter_C|SetIsInside _asbp_shooting_character false)))

(event EventBeginPlay
  (bind _asbp_shooting_character (Utilities|Casting|CastToBP_ShootingCharacter (Game|GetPlayerCharacter 0)))
  (Default|FuncDealMagneticField _asbp_shooting_character)
  (Utilities|FlowControl|Delay 0.2)
  (Variables|/Script/Engine.PrimitiveComponent|SetbGenerateOverlapEvents (Variables|Default|GetStaticMesh) true)
  (bind _shrink (Timeline|Shrink Play)
    (:Update
      (Transformation|SetWorldScale3D (Variables|Default|GetStaticMesh) (Math|Vector|MakeVector _shrink _shrink 5e+03)))))

(fn ConstructionScript)

(fn SetField
  (Variables|Default|SetOldLoc (Transformation|GetActorLocation))
  (Variables|Default|SetNewLoc (+ (Math|Vector|MakeVector (Math|Random|RandomFloatinRange -1e+03 1e+03) (Math|Random|RandomFloatinRange -1e+03 1e+03) 0.0) (Transformation|GetActorLocation)))
  (Variables|Default|SetScale (Transformation|GetWorldScale (Variables|Default|GetStaticMesh))))

(fn UpdateField
  (params (Lerp :type Float%20%28single-precision%29))
  (Transformation|SetWorldScale3D (Variables|Default|GetStaticMesh) (Math|Vector|Lerp(Vector) (Variables|Default|GetScale) (- (Variables|Default|GetScale) (Variables|Default|GetShrinkAmount)) Lerp))
  (Transformation|SetActorLocation (Math|Vector|Lerp(Vector) (Variables|Default|GetOldLoc) (Variables|Default|GetNewLoc) Lerp) false false))